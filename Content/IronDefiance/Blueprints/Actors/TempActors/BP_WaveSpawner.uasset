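; BP_WaveSpawner is an actor that spawns waves of BP_TempEnemy at its arrow component, passing each a Target and itself.
; SpawnEnemy, called shortly after BeginPlay, starts a looping timer with one randomized interval.
; Spawn counts enemies up to the wave quota, then clears the timer, raises the quota and increments CurrentWave, without restarting the timer itself.
; OnSpawnedAIDeath removes destroyed enemies and updates EnemiesOnField.
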(event `self.ReceiveBeginPlay`
  (`KismetSystemLibrary.Delay` 1.0)
  (`self.SpawnEnemy`))

(event `SpawnEnemy`
  (bind _time (`self.Time`))
  (bind _returnvalue (`KismetSystemLibrary.K2_SetTimerDelegate` (delegate `Spawn`) (`KismetMathLibrary.RandomFloatInRange` _time (* _time 1.5)) true))
  (set `self.NewVar` _returnvalue))

(event `Spawn`
  (bind _spawnenemies (`self.SpawnEnemies`))
  (bind _arrow (`self.Arrow`))
  (if (>= (`self.EnemiesSpawned`) (`self.EnemiesToSpawn`))
    (`KismetSystemLibrary.K2_ClearAndInvalidateTimerHandle` (`self.NewVar`))
    (set `self.EnemiesSpawned` 0)
    (set `self.EnemiesToSpawn` (+ (`self.EnemiesToSpawn`) 3))
    (`/Engine/EditorBlueprintResources/StandardMacros.IncrementInt` (`self.CurrentWave`))
    (else
      (bind _returnvalue (`|SpawnActorFromClass` "/Game/IronDefiance/Blueprints/Actors/TempActors/BP_TempEnemy.BP_TempEnemy_C" (`KismetMathLibrary.MakeTransform` (`SceneComponent.K2_GetComponentLocation` _arrow) (`SceneComponent.K2_GetComponentRotation` _arrow)) "AdjustIfPossibleButAlwaysSpawn" "MultiplyWithRoot" null (`self.Target`) self 50.0 null))
      (`KismetArrayLibrary.Array_AddUnique` _spawnenemies _returnvalue)
      (set `self.EnemiesOnField` (+ (`KismetArrayLibrary.Array_LastIndex` _spawnenemies) 1))
      (`/Engine/EditorBlueprintResources/StandardMacros.IncrementInt` (`self.EnemiesSpawned`)))))

(event `/Game/IronDefiance/Blueprints/Actors/TempActors/BPI_Spawner.OnSpawnedAIDeath`
  (params (AIDestroyed :type "Actor Object Reference"))
  (bind _spawnenemies (`self.SpawnEnemies`))
  (bind _returnvalue (`KismetArrayLibrary.Array_LastIndex` _spawnenemies))
  (bind _returnvalue_2 (`KismetArrayLibrary.Array_RemoveItem` (`self.SpawnEnemies`) AIDestroyed))
  (if _returnvalue_2
    (if (`KismetArrayLibrary.Array_IsValidIndex` _spawnenemies _returnvalue)
      (set `self.EnemiesOnField` (+ _returnvalue 1))
      (else
        (set `self.EnemiesOnField` 0)))))

(fn `UserConstructionScript`)