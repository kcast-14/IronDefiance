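; Temporary tank character that fights autonomously or under direct player control, switching back to operator mode on input.
; When possessed, it adds input mapping and a HUD, aims turret yaw by control rotation and clamped barrel pitch by camera trace, and fires bullets gated by a Tick-driven reload.
; Otherwise, AI perception picks an "Enemy"-tagged target, the turret tracks it, and a looping timer fires at the reload interval.
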(event `self.ReceiveBeginPlay`
  (bind _returnvalue (`GameplayStatics.GetActorOfClass` "/Game/IronDefiance/Blueprints/Actors/TempActors/Target.Target_C"))
  (set `self.DefendTarget` _returnvalue)
  (set `self.ReloadTime` (`self.ReloadTimer`))
  (set `self.SpawnLoc` (`self.K2_GetActorLocation`))
  (set `self.SpawnRot` (`self.K2_GetActorRotation`)))

(event `self.ReceivePossessed`
  (params (NewController :type "Controller Object Reference"))
  (if (== NewController (`GameplayStatics.GetPlayerController` 0))
    (set `self.Playercontrolled?` true)
    (bind _asbp_player_controller (cast `/Game/IronDefiance/Blueprints/Controllers/PlayerController/BP_PlayerController` (`self.GetController`)))
    (bind _returnvalue (pcsubsystem `EnhancedInputLocalPlayerSubsystem` _asbp_player_controller))
    (`/Engine/EditorBlueprintResources/StandardMacros.IsValid` _returnvalue
      (:`Is Valid`
        (`EnhancedInputSubsystemInterface.AddMappingContext` _returnvalue "/Game/IronDefiance/Blueprints/Input/IM_PlayerMapping.IM_PlayerMapping" 0 (struct))
        (set `PlayerController.bShowMouseCursor` false (`GameplayStatics.GetPlayerController` 0))
        (bind _returnvalue_2 (`|CreateWidget` "/Game/IronDefiance/UI/Widgets/TempHud/W_TempActionHUD.W_TempActionHUD_C"))
        (`UserWidget.AddToViewport` _returnvalue_2 0)
        (set `self.HudRef` _returnvalue_2)))))

(event `EnhancedInput|/Game/IronDefiance/Blueprints/Input/InputAction/SwitchToOperator`
  (params (ActionValue :type Boolean) (ElapsedSeconds :type "Float (double-precision)") (TriggeredSeconds :type "Float (double-precision)") (InputAction :type "InputAction Object Reference" :default "/Game/IronDefiance/Blueprints/Input/InputAction/SwitchToOperator.SwitchToOperator"))
  (:`Triggered`
    (bind _operatormoderef (`self.OperatorModeRef`)
      (:`then`
        (`Controller.Possess` (`GameplayStatics.GetPlayerController` 0) _operatormoderef)
        (set `self.OperatorModeRef` null)
        (`|ExecutionSequence`
          (:`then_0`
            (set `self.Playercontrolled?` false)
            (`Widget.RemoveFromParent` (stale `self.ReceivePossessed` _returnvalue_2))
            (bind _aicontroller (`self.AIController`)
              (:`then`
                (`Controller.Possess` _aicontroller self)
                (`KismetSystemLibrary.Delay` 0.5))
              (:`else`)))))
      (:`else`))))

(event `EnhancedInput|/Game/IronDefiance/Blueprints/Input/InputAction/Movement`
  (params (ActionValue :type "Vector2D Structure") (ElapsedSeconds :type "Float (double-precision)") (TriggeredSeconds :type "Float (double-precision)") (InputAction :type "InputAction Object Reference" :default "/Game/IronDefiance/Blueprints/Input/InputAction/Movement.Movement"))
  (bind _cube (`self.Cube`))
  (bind (_returnvalue_roll _returnvalue_pitch _returnvalue_yaw) (`KismetMathLibrary.BreakRotator` (`SceneComponent.K2_GetComponentRotation` _cube)))
  (:`Triggered`
    (`SceneComponent.K2_SetWorldRotation` _cube (`KismetMathLibrary.MakeRotator` 0.0 0.0 (+ ActionValue_X _returnvalue_yaw)) false false)
    (`self.AddMovementInput` (`SceneComponent.GetForwardVector` (`self.Cube`)) ActionValue_Y)))

(event `EnhancedInput|/Game/IronDefiance/Blueprints/Input/InputAction/Look`
  (params (ActionValue :type "Vector2D Structure") (ElapsedSeconds :type "Float (double-precision)") (TriggeredSeconds :type "Float (double-precision)") (InputAction :type "InputAction Object Reference" :default "/Game/IronDefiance/Blueprints/Input/InputAction/Look.Look"))
  (:`Triggered`
    (`self.AddControllerYawInput` ActionValue_X)
    (`self.AddControllerPitchInput` (* ActionValue_Y -1.0))))

(event `EnhancedInput|/Game/IronDefiance/Blueprints/Input/InputAction/ZoomOut`
  (params (ActionValue :type "Float (double-precision)") (ElapsedSeconds :type "Float (double-precision)") (TriggeredSeconds :type "Float (double-precision)") (InputAction :type "InputAction Object Reference" :default "/Game/IronDefiance/Blueprints/Input/InputAction/ZoomOut.ZoomOut"))
  (bind _springarm (`self.SpringArm`))
  (bind _springarm1 (`self.SpringArm1`))
  (:`Triggered`
    (set `SpringArmComponent.TargetArmLength` (`KismetMathLibrary.FClamp` (+ (* ActionValue (`self.ZoomSpeed`)) (`SpringArmComponent.TargetArmLength` _springarm)) 50.0 600.0) _springarm)
    (set `SpringArmComponent.TargetArmLength` (`KismetMathLibrary.FClamp` (+ ActionValue (`SpringArmComponent.TargetArmLength` _springarm1)) 0.0 100.0) _springarm1)))

(event `EnhancedInput|/Game/IronDefiance/Blueprints/Input/InputAction/LMB`
  (params (ActionValue :type Boolean) (ElapsedSeconds :type "Float (double-precision)") (TriggeredSeconds :type "Float (double-precision)") (InputAction :type "InputAction Object Reference" :default "/Game/IronDefiance/Blueprints/Input/InputAction/LMB.LMB"))
  (bind (_returnvalue_location _returnvalue_rotation) (`KismetMathLibrary.BreakTransform` (`SceneComponent.K2_GetComponentToWorld` (`self.BulletSpawn`))))
  (:`Triggered`
    (if (`self.CanShoot`)
      (set `self.ReloadTime` 0.0)
      (set `self.ShootTimer` (struct))
      (`|SpawnActorFromClass` "/Game/IronDefiance/Blueprints/Actors/TempActors/BP_Bullet.BP_Bullet_C" (`KismetMathLibrary.MakeTransform` _returnvalue_location _returnvalue_rotation) "AlwaysSpawn" "MultiplyWithRoot" null (`self.AverageDamage`) self self)
      (set `self.CanShoot` false))))

(event `EnhancedInput|/Game/IronDefiance/Blueprints/Input/InputAction/Pause`
  (params (ActionValue :type Boolean) (ElapsedSeconds :type "Float (double-precision)") (TriggeredSeconds :type "Float (double-precision)") (InputAction :type "InputAction Object Reference" :default "/Game/IronDefiance/Blueprints/Input/InputAction/Pause.Pause"))
  (:`Triggered`
    (`/Engine/EditorBlueprintResources/StandardMacros.FlipFlop`
      (:`A`
        (`GameplayStatics.SetGamePaused` true)
        (set `PlayerController.bShowMouseCursor` true (`GameplayStatics.GetPlayerController` 0))
        (bind _returnvalue (`|CreateWidget` "/Game/IronDefiance/UI/Widgets/TempHud/W_Pause.W_Pause_C"))
        (`UserWidget.AddToViewport` _returnvalue 0))
      (:`B`
        (`GameplayStatics.SetGamePaused` false)
        (set `PlayerController.bShowMouseCursor` false (`GameplayStatics.GetPlayerController` 0))
        (`Widget.RemoveFromParent` _returnvalue)))))

(event `EnhancedInput|/Game/IronDefiance/Blueprints/Input/InputAction/ZoomIn`
  (params (ActionValue :type "Float (double-precision)") (ElapsedSeconds :type "Float (double-precision)") (TriggeredSeconds :type "Float (double-precision)") (InputAction :type "InputAction Object Reference" :default "/Game/IronDefiance/Blueprints/Input/InputAction/ZoomIn.ZoomIn"))
  (bind _springarm (`self.SpringArm`))
  (bind _springarm1 (`self.SpringArm1`))
  (:`Triggered`
    (set `SpringArmComponent.TargetArmLength` (`KismetMathLibrary.FClamp` (- (`SpringArmComponent.TargetArmLength` _springarm) (* ActionValue (`self.ZoomSpeed`))) 50.0 600.0) _springarm)
    (set `SpringArmComponent.TargetArmLength` (`KismetMathLibrary.FClamp` (- (`SpringArmComponent.TargetArmLength` _springarm1) ActionValue) 0.0 100.0) _springarm1)))

(event `self.ReceiveTick`
  (params (DeltaSeconds :type "Float (single-precision)"))
  (bind (_returnvalue_location _returnvalue_rotation) (`KismetMathLibrary.BreakTransform` (`SceneComponent.K2_GetComponentToWorld` (`self.BulletSpawn`))))
  (bind (_returnvalue_roll _returnvalue_pitch _returnvalue_yaw) (`KismetMathLibrary.BreakRotator` (`SceneComponent.K2_GetComponentRotation` (`self.Cylinder`))))
  (set `self.Delta Seconds` DeltaSeconds)
  (`|ExecutionSequence`
    (:`then_0`
      (if (`self.Playercontrolled?`)
        (bind _outhit (`self.LineTraceForCam`))
        (`self.BarrelRotation` _outhit (`self.Delta Seconds`) 8.0)
        (`self.TurretRotation` (`self.Delta Seconds`) 8.0)
        (bind _hudref (`self.HudRef`)
          (:`then`
            (`/Game/IronDefiance/UI/Widgets/TempHud/W_TempActionHUD.SetReloadProg` _hudref (/ (`self.ReloadTime`) (`self.ReloadTimer`))))
          (:`else`))
        (else
          (bind _curenttarget (`self.CurentTarget`)
            (:`then`
              (bind (_returnvalue_roll_2 _returnvalue_pitch_2 _returnvalue_yaw_2) (`KismetMathLibrary.BreakRotator` (`KismetMathLibrary.FindLookAtRotation` (`SceneComponent.K2_GetComponentLocation` (`self.Cylinder`)) (`self.K2_GetActorLocation` _curenttarget))))
              (bind (_returnvalue_roll_3 _returnvalue_pitch_3 _returnvalue_yaw_3) (`KismetMathLibrary.BreakRotator` (`KismetMathLibrary.RInterpTo` (`KismetMathLibrary.MakeRotator` 0.0 0.0 _returnvalue_yaw) (`KismetMathLibrary.MakeRotator` 0.0 0.0 _returnvalue_yaw_2) (`self.Delta Seconds`) 10.0)))
              (`SceneComponent.K2_SetWorldRotation` (`self.Cylinder`) (`KismetMathLibrary.MakeRotator` 0.0 0.0 _returnvalue_yaw_3) false false)
              (`/Engine/EditorBlueprintResources/StandardMacros.DoOnce` false :!label _label
                (:`Completed`
                  (`|ExecutionSequence`
                    (:`then_0`
                      (bind _returnvalue (`KismetSystemLibrary.K2_SetTimerDelegate` (delegate `Shoot`) (`self.ReloadTimer`) true))
                      (set `self.ShootTimer` _returnvalue))
                    (:`then_1`
                      (`/Engine/EditorBlueprintResources/StandardMacros.IsValid` (`self.CurentTarget`) :!label _label_2
                        (:`Is Valid`
                          (`|SpawnActorFromClass` "/Game/IronDefiance/Blueprints/Actors/TempActors/BP_Bullet.BP_Bullet_C" (`KismetMathLibrary.MakeTransform` _returnvalue_location _returnvalue_rotation) "AlwaysSpawn" "MultiplyWithRoot" null (`self.AverageDamage`) self self))
                        (:`Is Not Valid`
                          (`KismetSystemLibrary.K2_ClearAndInvalidateTimerHandle` (`self.ShootTimer`)))))))))
            (:`else`
              (goto _label :!via `Reset`))))))
    (:`then_1`
      (`self.ReloadFunction`))))

(event `Shoot`
  (goto _label_2))

(event `/Game/IronDefiance/Blueprints/Actors/TempActors/BPI_Tanks.UpdateTarget`
  (set `self.CurentTarget` null))

(event `self.AIPerception.OnTargetPerceptionUpdated`
  (params (Actor :type "Actor Object Reference") (Stimulus :type "AIStimulus Structure"))
  (`self.CurentTarget`
    (:`then`)
    (:`else`
      (if (`self.ActorHasTag` Actor "Enemy")
        (set `self.CurentTarget` Actor)))))

(fn `ReloadFunction`
  (if (not (`self.CanShoot`))
    (set `self.ReloadTime` (`KismetMathLibrary.FClamp` (+ (`self.Delta Seconds`) (`self.ReloadTime`)) 0.0 (`self.ReloadTimer`)))
    (if (== (`self.ReloadTime`) (`self.ReloadTimer`))
      (set `self.CanShoot` true))))

(fn `UserConstructionScript`)