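; BP_Bullet is a temporary projectile Blueprint with leftover hit logic for damaging enemies, none of which is connected to a live event.
; The disconnected logic skips itself and Tower-tagged actors, damages Enemy-tagged actors with the instigator as causer, and destroys the bullet unless the other actor is tagged Ignore.
; CalculateDamage is meant to supply the damage, but contains only an unused random-range calculation.
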(fn `UserConstructionScript`)