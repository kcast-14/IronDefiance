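; BP_TempEnemy is a temporary enemy actor with health that takes damage and destroys itself at zero HP.
; Tick turns its HP widget toward the player camera and pushes current and max HP to it every frame.
; Lethal damage sends an update-target message to the instigator before destruction.
; EndPlay, given a valid Spawner, reports the death to it and fires the enemy-destroyed call.
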(event `self.ReceiveBeginPlay`
  (set `self.CurrentHP` (`self.MaxHP`)))

(event `self.ReceiveEndPlay`
  (params (EndPlayReason :type "EEndPlayReason Enum" :default "Destroyed"))
  (bind _spawner (`self.Spawner`)
    (:`then`
      (message `/Game/IronDefiance/Blueprints/Actors/TempActors/BPI_Spawner.OnSpawnedAIDeath` _spawner self)
      (`self.OnEnemyDestroyed`))
    (:`else`)))

(event `self.ReceiveTick`
  (params (DeltaSeconds :type "Float (single-precision)"))
  (`SceneComponent.K2_SetWorldRotation` (`self.Widget`) (`KismetMathLibrary.FindLookAtRotation` (`SceneComponent.K2_GetComponentLocation` (`self.Widget`)) (`PlayerCameraManager.GetCameraLocation` (`GameplayStatics.GetPlayerCameraManager` 0))) false false)
  (message `/Game/IronDefiance/Blueprints/Actors/TempActors/BPI_HPBar.HPUpdate` (`WidgetComponent.GetWidget` (`self.Widget`)) (`self.MaxHP`) (`self.CurrentHP`)))

(event `self.ReceiveAnyDamage`
  (params (Damage :type "Float (single-precision)") (DamageType :type "DamageType Object Reference") (InstigatedBy :type "Controller Object Reference") (DamageCauser :type "Actor Object Reference"))
  (if (> (`self.CurrentHP`) 0.0)
    (bind _output_get (set `self.CurrentHP` (- (`self.CurrentHP`) Damage)))
    (if (<= _output_get 0.0)
      (`self.Death` InstigatedBy))))

(event `Death`
  (params (DmgCauser :type "Actor Object Reference"))
  (message `/Game/IronDefiance/Blueprints/Actors/TempActors/BPI_Tanks.UpdateTarget` DmgCauser)
  (`self.K2_DestroyActor`))

(fn `UserConstructionScript`)