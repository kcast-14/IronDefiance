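; BP_TempPlayer is a temporary operator-mode player character that places tanks in the level or takes control of placed ones.
; Possession and BeginPlay set up input mapping, cursor and HUD, movement input offsets the actor directly, and a pause action toggles a menu.
; Clicks trace from the cursor to spawn the tank chosen through SetTank, blocking "Tower"-tagged targets, or with none selected possess the clicked tank, passing it a reference back.
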(event `self.ReceivePossessed`
  (params (NewController :type "Controller Object Reference"))
  (bind _asbp_player_controller (cast `/Game/IronDefiance/Blueprints/Controllers/PlayerController/BP_PlayerController` (`self.GetController`) :!label _label))
  (bind _returnvalue (pcsubsystem `EnhancedInputLocalPlayerSubsystem` _asbp_player_controller))
  (`/Engine/EditorBlueprintResources/StandardMacros.IsValid` _returnvalue
    (:`Is Valid`
      (`EnhancedInputSubsystemInterface.AddMappingContext` _returnvalue "/Game/IronDefiance/Blueprints/Input/IM_PlayerMapping.IM_PlayerMapping" 0 (struct))
      (set `PlayerController.bShowMouseCursor` true (`GameplayStatics.GetPlayerController` 0))
      (bind _returnvalue_2 (`|CreateWidget` "/Game/IronDefiance/UI/Widgets/TempHud/W_TempHUD.W_TempHUD_C"))
      (bind _output_get (set `self.HUDRef` _returnvalue_2))
      (`UserWidget.AddToViewport` _output_get 0))))

(event `self.ReceiveBeginPlay`
  (goto _label))

(event `self.ReceiveUnpossessed`
  (params (OldController :type "Controller Object Reference"))
  (`Widget.RemoveFromParent` (stale `self.ReceivePossessed` _output_get)))

(event `EnhancedInput|/Game/IronDefiance/Blueprints/Input/InputAction/MovementOperator`
  (params (ActionValue :type "Vector2D Structure") (ElapsedSeconds :type "Float (double-precision)") (TriggeredSeconds :type "Float (double-precision)") (InputAction :type "InputAction Object Reference" :default "/Game/IronDefiance/Blueprints/Input/InputAction/MovementOperator.MovementOperator"))
  (bind _maxwalkspeed (`CharacterMovementComponent.MaxWalkSpeed` (`self.CharacterMovement`)))
  (:`Triggered`
    (`self.K2_AddActorWorldOffset` (`KismetMathLibrary.MakeVector` (* ActionValue_Y _maxwalkspeed) (* ActionValue_X _maxwalkspeed)))))

(event `EnhancedInput|/Game/IronDefiance/Blueprints/Input/InputAction/Pause`
  (params (ActionValue :type Boolean) (ElapsedSeconds :type "Float (double-precision)") (TriggeredSeconds :type "Float (double-precision)") (InputAction :type "InputAction Object Reference" :default "/Game/IronDefiance/Blueprints/Input/InputAction/Pause.Pause"))
  (:`Triggered`
    (`/Engine/EditorBlueprintResources/StandardMacros.FlipFlop`
      (:`A`
        (`GameplayStatics.SetGamePaused` true)
        (set `PlayerController.bShowMouseCursor` true (`GameplayStatics.GetPlayerController` 0))
        (bind _returnvalue (`|CreateWidget` "/Game/IronDefiance/UI/Widgets/TempHud/W_Pause.W_Pause_C"))
        (`UserWidget.AddToViewport` _returnvalue 0))
      (:`B`
        (`GameplayStatics.SetGamePaused` false)
        (set `PlayerController.bShowMouseCursor` true (`GameplayStatics.GetPlayerController` 0))
        (`Widget.RemoveFromParent` _returnvalue)))))

(event `EnhancedInput|/Game/IronDefiance/Blueprints/Input/InputAction/LMB`
  (params (ActionValue :type Boolean) (ElapsedSeconds :type "Float (double-precision)") (TriggeredSeconds :type "Float (double-precision)") (InputAction :type "InputAction Object Reference" :default "/Game/IronDefiance/Blueprints/Input/InputAction/LMB.LMB"))
  (bind (_worldlocation _worlddirection) (`PlayerController.DeprojectMousePositionToWorld` (`GameplayStatics.GetPlayerController` 0)))
  (:`Triggered`
    (bind (_outhit _returnvalue) (`KismetSystemLibrary.LineTraceSingle` _worldlocation (+ _worldlocation (* _worlddirection 10000.0)) "TraceTypeQuery1"))
    (if _returnvalue
      (bind _tanktoplace (`self.TankToPlace`)
        (:`then`
          (bind (_bblockinghit _binitialoverlap _time _distance _location _impactpoint _normal _impactnormal _physmat _hitactor) (`GameplayStatics.BreakHitResult` _outhit))
          (if (`self.ActorHasTag` _hitactor "Tower")
            (`KismetSystemLibrary.PrintString` "Cannot Spawn on top of another tank")
            (else
              (`|SpawnActorFromClass` _tanktoplace (`KismetMathLibrary.MakeTransform` _location) "AdjustIfPossibleButAlwaysSpawn" "MultiplyWithRoot" null null)
              (message `/Game/IronDefiance/Blueprints/Actors/TempActors/BPI_HUD.DisableButton` (`self.HUDRef`) (`self.Button Used`)))))
        (:`else`
          (if (`self.ActorHasTag` _hitactor "Tower")
            (bind _asbp_temp_tanks (cast `/Game/IronDefiance/Blueprints/Characters/AI/TankAI/BP_TempTanks` _hitactor))
            (set `/Game/IronDefiance/Blueprints/Characters/AI/TankAI/BP_TempTanks.OperatorModeRef` self _asbp_temp_tanks)
            (`Controller.Possess` (`GameplayStatics.GetPlayerController` 0) _asbp_temp_tanks)))))))

(event `/Game/IronDefiance/Blueprints/Characters/Player/TempBP/NewFolder/BPI_TempPlayer.SetTank`
  (params (Tank :type "Actor Class Reference") (ButtonUsed :type "Button Object Reference"))
  (set `self.TankToPlace` Tank)
  (set `self.Button Used` ButtonUsed))

(fn `UserConstructionScript`)