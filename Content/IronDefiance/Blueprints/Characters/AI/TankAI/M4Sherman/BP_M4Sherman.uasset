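; Player-driven M4 Sherman tank pawn with Enhanced Input for driving, turning and camera orbit.
; Each tick averages hits from BP_GroundSensing components to align the hull to terrain and set its height, moving it by interpolated transforms without sweep.
; A camera line trace sets the aim point for clamped, interpolated barrel pitch.
; Turret rotation interpolates with no target wired, leaving the spring-arm yaw rotator unused.
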(event `self.ReceiveBeginPlay`
  (`EnhancedInputSubsystemInterface.AddMappingContext` (pcsubsystem `EnhancedInputLocalPlayerSubsystem` (`GameplayStatics.GetPlayerController` 0)) "/Game/IronDefiance/Blueprints/Input/IM_TankMapping.IM_TankMapping" 0 (struct))
  (set `self.GroundSensing` (`self.K2_GetComponentsByClass` "/Game/IronDefiance/Blueprints/Characters/AI/TankAI/BP_GroundSensing.BP_GroundSensing_C")))

(event `self.ReceiveTick`
  (params (DeltaSeconds :type "Float (single-precision)"))
  (bind _returnvalue (`GameplayStatics.GetWorldDeltaSeconds`))
  (bind (_returnvalue_x _returnvalue_y _returnvalue_z) (`KismetMathLibrary.BreakVector` (`self.K2_GetActorLocation`)))
  (bind _returnvalue_2 (`KismetMathLibrary.FInterpTo` (`self.CurrentForwardSpeed`) (`self.TargetForwardSpeed`) _returnvalue 2.0))
  (`|ExecutionSequence`
    (:`then_0`
      (set `self.AverageNormal` (0.0 0.0 0.0))
      (set `self.AverageHeight` 0.0)
      (set `self.CountOnGround` 0))
    (:`then_1`
      (for _array_element (`self.GroundSensing`)
        (if (`/Game/IronDefiance/Blueprints/Characters/AI/TankAI/BP_GroundSensing.bOnGround` _array_element)
          (`/Engine/EditorBlueprintResources/StandardMacros.IncrementInt` (`self.CountOnGround`)
            (:`  `
              (set `self.AverageNormal` (+ (`/Game/IronDefiance/Blueprints/Characters/AI/TankAI/BP_GroundSensing.HitNormal` _array_element) (`self.AverageNormal`)))
              (bind (_hitloc_x _hitloc_y _hitloc_z) (`KismetMathLibrary.BreakVector` (`/Game/IronDefiance/Blueprints/Characters/AI/TankAI/BP_GroundSensing.HitLoc` _array_element)))
              (set `self.AverageHeight` (+ _hitloc_z (`self.AverageHeight`)))))))
      (set `self.AverageNormal` (/ (`self.AverageNormal`) (`self.CountOnGround`)))
      (bind _output_get (set `self.AverageHeight` (/ (`self.AverageHeight`) (`self.CountOnGround`))))
      (set `self.DeltaZ` (- (+ _output_get (`self.HeightOffSet`)) _returnvalue_z))
      (`self.K2_SetActorRotation` (`KismetMathLibrary.RInterpTo` (`self.K2_GetActorRotation`) (`KismetMathLibrary.ComposeRotators` (`KismetMathLibrary.MakeRotator` 0.0 0.0 (* (`self.TargetTurnSpeed`) (`GameplayStatics.GetWorldDeltaSeconds`))) (`KismetMathLibrary.MakeRotFromZY` (`self.AverageNormal`) (`self.GetActorRightVector`))) (`GameplayStatics.GetWorldDeltaSeconds`) 8.0))
      (`self.K2_AddActorWorldOffset` (+ (* (`self.GetActorForwardVector`) _returnvalue_2 _returnvalue) (* (`self.GetActorUpVector`) (`self.DeltaZ`))))
      (set `self.CurrentForwardSpeed` _returnvalue_2))
    (:`then_2`
      (bind _outhit (`self.CameraTrace`))
      (`self.BarrelMovement` _outhit)
      (`self.TurretMovement`))))

(event `EnhancedInput|/Game/IronDefiance/Blueprints/Input/InputAction/Tank/Drive`
  (params (ActionValue :type "Float (double-precision)") (ElapsedSeconds :type "Float (double-precision)") (TriggeredSeconds :type "Float (double-precision)") (InputAction :type "InputAction Object Reference" :default "/Game/IronDefiance/Blueprints/Input/InputAction/Tank/Drive.Drive"))
  (:`Triggered`
    (set `self.TargetForwardSpeed` (* ActionValue (`self.MaxForwardSpeed`))))
  (:`Completed`
    (set `self.TargetForwardSpeed` 0.0)))

(event `EnhancedInput|/Game/IronDefiance/Blueprints/Input/InputAction/Tank/Turn`
  (params (ActionValue :type "Float (double-precision)") (ElapsedSeconds :type "Float (double-precision)") (TriggeredSeconds :type "Float (double-precision)") (InputAction :type "InputAction Object Reference" :default "/Game/IronDefiance/Blueprints/Input/InputAction/Tank/Turn.Turn"))
  (:`Triggered`
    (set `self.TargetTurnSpeed` (* ActionValue (`self.MaxTurnSpeed`))))
  (:`Completed`
    (set `self.TargetTurnSpeed` 0.0)))

(event `EnhancedInput|/Game/IronDefiance/Blueprints/Input/InputAction/Tank/Look`
  (params (ActionValue :type "Vector2D Structure") (ElapsedSeconds :type "Float (double-precision)") (TriggeredSeconds :type "Float (double-precision)") (InputAction :type "InputAction Object Reference" :default "/Game/IronDefiance/Blueprints/Input/InputAction/Tank/Look.Look"))
  (bind _springarm (`self.SpringArm`))
  (:`Triggered`
    (`SceneComponent.K2_AddRelativeRotation` _springarm (`KismetMathLibrary.MakeRotator` 0.0 0.0 (`KismetMathLibrary.NormalizeAxis` ActionValue_X)) false false)
    (`SceneComponent.K2_AddRelativeRotation` _springarm (`KismetMathLibrary.MakeRotator` 0.0 (`KismetMathLibrary.NormalizeAxis` ActionValue_Y)) false false)))

(fn `UserConstructionScript`)