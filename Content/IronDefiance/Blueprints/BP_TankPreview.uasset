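; BP_TankPreview is a tank placement preview that tracks whether its spot is valid.
; Box overlaps with "invalid"-tagged actors are stored in OverlappingActors and clear ValidPlacement, which returns to true when an end overlap leaves the list empty.
; Both handlers call CheckValid to set a green or red mesh material, but its branch ignores the Valid input and is fixed true, so it always applies green.
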(event `self.Box.OnComponentBeginOverlap`
  (params (OverlappedComponent :type "PrimitiveComponent Object Reference") (OtherActor :type "Actor Object Reference") (OtherComp :type "PrimitiveComponent Object Reference") (OtherBodyIndex :type Integer) (bFromSweep :type Boolean) (SweepResult :type "HitResult Structure (by ref)"))
  (if (`self.ActorHasTag` OtherActor "invalid")
    (`KismetArrayLibrary.Array_Add` (`self.OverlappingActors`) OtherActor)
    (bind _output_get (set `self.ValidPlacement` false))
    (`self.CheckValid` _output_get)))

(event `self.Box.OnComponentEndOverlap`
  (params (OverlappedComponent :type "PrimitiveComponent Object Reference") (OtherActor :type "Actor Object Reference") (OtherComp :type "PrimitiveComponent Object Reference") (OtherBodyIndex :type Integer))
  (`KismetArrayLibrary.Array_RemoveItem` (`self.OverlappingActors`) OtherActor)
  (if (`KismetArrayLibrary.Array_IsEmpty` (`self.OverlappingActors`))
    (bind _output_get (set `self.ValidPlacement` true))
    (`self.CheckValid` _output_get)))

(fn `CheckValid`
  (params (`Valid?` :type Boolean))
  (if true
    (`PrimitiveComponent.SetMaterial` (`self.StaticMesh`) 0 "/AnimationSharing/AnimSharingGreen.AnimSharingGreen")
    (else
      (`PrimitiveComponent.SetMaterial` (`self.StaticMesh`) 0 "/AnimationSharing/AnimSharingRed.AnimSharingRed"))))

(fn `UserConstructionScript`)