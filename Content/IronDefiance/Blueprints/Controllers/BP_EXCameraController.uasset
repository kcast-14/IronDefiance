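; Player controller for a top-down camera pawn that can toggle to possessing a BP_TestCharacter (FPSCam) spawned at BeginPlay.
; Switching moves the incoming pawn to the outgoing one's location before possessing it.
; Screen-edge cursor and axis input move the controlled pawn relative to its rotation, without mode checks or delta-time scaling.
; Rotation input yaws that pawn by delta time; zoom adjusts the camera pawn's spring arm length.
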(event `InputAction|SwitchCameraMode`
  (params (Key :type "Key Structure"))
  (bind _fpscam (`self.FPSCam`))
  (bind _as_bp_camera_extra (`self.As BP Camera Extra`))
  ;[1 1 1] Switch between modes
  (:`Pressed`
    (`|ExecutionSequence`
      (:`then_0`
        (if (`self.TopDown?`)
          (`self.K2_SetActorLocation` _fpscam (`self.K2_GetActorLocation` _as_bp_camera_extra) false false)
          (`self.Possess` _fpscam)
          (else
            (`self.K2_SetActorLocation` _as_bp_camera_extra (`self.K2_GetActorLocation` _fpscam) false false)
            (`self.Possess` _as_bp_camera_extra))))
      (:`then_1`
        (set `self.TopDown?` (not (`self.TopDown?`)))))))

(event `self.ReceiveBeginPlay`
  ;[1 1 1] Initialization
  (bind _asbp_camera_extra (cast `/Game/IronDefiance/Blueprints/BP_CameraExtra` (`self.K2_GetPawn`)))
  (bind _output_get (set `self.As BP Camera Extra` _asbp_camera_extra))
  (set `self.Spring Arm` (`/Game/IronDefiance/Blueprints/BP_CameraExtra.SpringArm` _output_get))
  (bind _returnvalue (`|SpawnActorFromClass` "/Game/IronDefiance/Blueprints/BP_TestCharacter.BP_TestCharacter_C" (`self.GetTransform` _output_get) "Undefined" "MultiplyWithRoot" null null))
  (set `self.FPSCam` _returnvalue))

(event `self.ReceiveTick`
  (params (DeltaSeconds :type "Float (single-precision)"))
  (bind _cameraedgescrollthreshold (`self.CameraEdgeScrollThreshold`))
  ;[0.4886 1 0.9701] Move By Mouse Cursor
  (bind _returnvalue (`WidgetLayoutLibrary.GetMousePositionOnViewport`))
  (bind _returnvalue_2 (`WidgetLayoutLibrary.GetViewportWidgetGeometry`))
  (`|ExecutionSequence`
    (:`then_0`
      (bind (_x _y) (`KismetMathLibrary.BreakVector2D` _returnvalue))
      (if (< _x _cameraedgescrollthreshold)
        (`self.MoveCamera` (`KismetMathLibrary.MakeVector` 0.0 (`self.CameraScrollSpeed`)))
        (else
          (bind (_x_2 _y_2) (`KismetMathLibrary.BreakVector2D` (`SlateBlueprintLibrary.GetLocalSize` _returnvalue_2)))
          (if (> _x (- _x_2 _cameraedgescrollthreshold))
            (`self.MoveCamera` (`KismetMathLibrary.MakeVector` 0.0 (* (`self.CameraScrollSpeed`) -1.0)))))))
    (:`then_1`
      (if (< _y (`self.CameraEdgeScrollThreshold`))
        (`self.MoveCamera` (`KismetMathLibrary.MakeVector` (* (`self.CameraScrollSpeed`) -1.0)))
        (elif (> _y (- _y_2 (`self.CameraEdgeScrollThreshold`)))
          (`self.MoveCamera` (`KismetMathLibrary.MakeVector` (`self.CameraScrollSpeed`))))))))

(event `InputAxis|Move Forward / Backward`
  (params (AxisValue :type "Float (single-precision)"))
  ;[1 1 1] Move by WASD
  (`self.MoveCamera` (`KismetMathLibrary.MakeVector` (* AxisValue (`self.CameraScrollSpeed`) -1.0))))

(event `InputAxis|Move Right / Left`
  (params (AxisValue :type "Float (single-precision)"))
  ;[1 1 1] Move by WASD
  (`self.MoveCamera` (`KismetMathLibrary.MakeVector` 0.0 (* AxisValue (`self.CameraScrollSpeed`) -1.0))))

(event `InputAction|ZoomIn`
  (params (Key :type "Key Structure"))
  ;[1 1 1] ZoomIn/Out
  (:`Pressed`
    (`self.CameraZoom` (* (`self.CameraZoomSpeed`) -1.0))))

(event `InputAction|ZoomOut`
  (params (Key :type "Key Structure"))
  ;[1 1 1] ZoomIn/Out
  (:`Pressed`
    (`self.CameraZoom` (`self.CameraZoomSpeed`))))

(event `InputAxis|RotateCamera`
  (params (AxisValue :type "Float (single-precision)"))
  ;[1 1 1] Rotate Camera
  (`self.RotateCameraLR` AxisValue))

(fn `CameraZoom`
  (params (B :type "Float (double-precision)"))
  (bind _spring_arm (`self.Spring Arm`))
  (set `SpringArmComponent.TargetArmLength` (+ (`SpringArmComponent.TargetArmLength` _spring_arm) B) _spring_arm))

(fn `MoveCamera`
  (params (B :type "Vector Structure"))
  (bind _returnvalue (`self.K2_GetPawn`))
  (`self.K2_SetActorLocation` _returnvalue (+ (`self.K2_GetActorLocation` _returnvalue) (`KismetMathLibrary.GreaterGreater_VectorRotator` B (`self.K2_GetActorRotation` _returnvalue))) false false))

(fn `RotateCameraLR`
  (params (A :type "Float (double-precision)"))
  (`self.K2_AddActorWorldRotation` (`self.K2_GetPawn`) (`KismetMathLibrary.MakeRotator` 0.0 0.0 (* A (`self.CameraRotationSpeed`) (`GameplayStatics.GetWorldDeltaSeconds`))) false false))

(fn `UserConstructionScript`)