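; Player controller for a top-down style camera, panning BP_CameraPawn with movement inputs and mouse screen edges.
; Each tick, MoveCamera combines normalized key input with edge offsets from viewport width (even vertically), scaled by a zoom-interpolated speed.
; Position clamps to 0–1 and pitch interpolates between zeros, so both look unfinished.
; Zoom inputs adjust a clamped alpha, but the spring-arm length update is disconnected and never runs.
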(event `self.ReceiveBeginPlay`
  (set `self.CameraPawn` (`GameplayStatics.GetPlayerPawn` 0))
  (`WidgetBlueprintLibrary.SetInputMode_GameAndUIEx` self null "LockAlways" false))

(event `self.ReceiveTick`
  (params (DeltaSeconds :type "Float (single-precision)"))
  (`self.MoveCamera`))

(event `InputAction|MoveLeft`
  (params (Key :type "Key Structure"))
  (bind _cameramovement (`self.CameraMovement`))
  ;[1 1 1] Movement
  (:`Pressed`
    (set `self.CameraMovement` (- _cameramovement (1.0 0.0 0.0))))
  (:`Released`
    (set `self.CameraMovement` (+ _cameramovement (1.0 0.0 0.0)))))

(event `InputAction|MoveForward`
  (params (Key :type "Key Structure"))
  (bind _cameramovement (`self.CameraMovement`))
  ;[1 1 1] Movement
  (:`Pressed`
    (set `self.CameraMovement` (- _cameramovement (0.0 1.0 0.0))))
  (:`Released`
    (set `self.CameraMovement` (+ _cameramovement (0.0 1.0 0.0)))))

(event `InputAction|MoveRight`
  (params (Key :type "Key Structure"))
  (bind _cameramovement (`self.CameraMovement`))
  ;[1 1 1] Movement
  (:`Pressed`
    (set `self.CameraMovement` (+ _cameramovement (1.0 0.0 0.0))))
  (:`Released`
    (set `self.CameraMovement` (- _cameramovement (1.0 0.0 0.0)))))

(event `InputAction|MoveDownward`
  (params (Key :type "Key Structure"))
  (bind _cameramovement (`self.CameraMovement`))
  ;[1 1 1] Movement
  (:`Pressed`
    (set `self.CameraMovement` (+ _cameramovement (0.0 1.0 0.0))))
  (:`Released`
    (set `self.CameraMovement` (- _cameramovement (0.0 1.0 0.0)))))

(event `EnhancedInput|/Game/IronDefiance/Blueprints/Input/InputAction/ZoomIn`
  (params (ActionValue :type Boolean) (ElapsedSeconds :type "Float (double-precision)") (TriggeredSeconds :type "Float (double-precision)") (InputAction :type "InputAction Object Reference" :default "/Game/IronDefiance/Blueprints/Input/InputAction/ZoomIn.ZoomIn"))
  ;[1 1 1] Zoom
  (:`Triggered`
    (set `self.CameraZoom` (`KismetMathLibrary.FClamp` (- (`self.CameraZoom`) 0.1)))))

(event `EnhancedInput|/Game/IronDefiance/Blueprints/Input/InputAction/ZoomOut`
  (params (ActionValue :type Boolean) (ElapsedSeconds :type "Float (double-precision)") (TriggeredSeconds :type "Float (double-precision)") (InputAction :type "InputAction Object Reference" :default "/Game/IronDefiance/Blueprints/Input/InputAction/ZoomOut.ZoomOut"))
  ;[1 1 1] Zoom
  (:`Triggered`
    (set `self.CameraZoom` (`KismetMathLibrary.FClamp` (+ (`self.CameraZoom`) 0.1)))))

(fn `MoveCamera`
  (locals (`Mouse X` :type "Float (double-precision)") (`Mouse Y` :type "Float (double-precision)"))
  (bind _returnvalue_x (`KismetMathLibrary.BreakVector2D` (`WidgetLayoutLibrary.GetViewportSize`)))
  (bind _returnvalue_x_2 (`KismetMathLibrary.BreakVector2D` (`WidgetLayoutLibrary.GetViewportSize`)))
  (bind _returnvalue_x_3 (`KismetMathLibrary.BreakVector2D` (`WidgetLayoutLibrary.GetViewportSize`)))
  (bind _returnvalue_x_4 (`KismetMathLibrary.BreakVector2D` (`WidgetLayoutLibrary.GetViewportSize`)))
  (bind _camerapawn (`self.CameraPawn`))
  (bind (_returnvalue_x_5 _returnvalue_y) (`KismetMathLibrary.BreakVector` (+ (`self.K2_GetActorLocation` _camerapawn) (* (- (`KismetMathLibrary.Normal` (`self.CameraMovement`)) (`KismetMathLibrary.MakeVector` (- (`KismetMathLibrary.FClamp` (`KismetMathLibrary.NormalizeToRange` (`local.Mouse X`) 0.0 (* _returnvalue_x_2 0.05))) 1.0)) (`KismetMathLibrary.MakeVector` (* (`KismetMathLibrary.FClamp` (`KismetMathLibrary.NormalizeToRange` (`local.Mouse X`) (* _returnvalue_x_3 0.95) _returnvalue_x_3)) -1.0)) (`KismetMathLibrary.MakeVector` 0.0 (- (`KismetMathLibrary.FClamp` (`KismetMathLibrary.NormalizeToRange` (`local.Mouse Y`) 0.0 (* _returnvalue_x 0.05))) 1.0)) (`KismetMathLibrary.MakeVector` 0.0 (* (`KismetMathLibrary.FClamp` (`KismetMathLibrary.NormalizeToRange` (`local.Mouse Y`) (* _returnvalue_x_4 0.95) _returnvalue_x_4)) -1.0))) (`KismetMathLibrary.Lerp` (`self.MincameraSpeed`) (`self.MaxCameraSpeed`) (`self.CameraZoom`))))))
  (bind _returnvalue (`WidgetLayoutLibrary.GetMousePositionOnViewport`))
  (set `local.Mouse X` (`KismetMathLibrary.BreakVector2D` _returnvalue))
  (set `local.Mouse Y` (`.Y` (`KismetMathLibrary.BreakVector2D` _returnvalue)))
  (`self.K2_SetActorLocationAndRotation` _camerapawn (`KismetMathLibrary.MakeVector` (`KismetMathLibrary.FClamp` _returnvalue_x_5) (`KismetMathLibrary.FClamp` _returnvalue_y)) (`KismetMathLibrary.MakeRotator` 0.0 (`KismetMathLibrary.Lerp` 0.0 0.0 (`self.CameraZoom`))) false false)
  ;[1 1 1] Zoom In/Out
  (bind _asbp_camera_pawn (cast `/Game/IronDefiance/Blueprints/BP_CameraPawn` (`self.CameraPawn`))))

(fn `UserConstructionScript`)